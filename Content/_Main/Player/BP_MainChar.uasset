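; Networked player character Blueprint handling movement, sprinting, rolling, a montage-based light attack and gear pickup.
; Server events gate rolls, attacks and interaction, with multicasts playing montages whose completion calls back to clear state.
; Sprint speed is set locally and on the server, while OnRep functions update animation and attach equipped weapon, shield or helmet to mesh sockets.
; Secondary input requests Blocking, which has no implementation.
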(event `self.ReceiveTick`
  (params (DeltaSeconds :type "Float (single-precision)"))
  (`parent.ReceiveTick` DeltaSeconds))

(event `InputAxis|Turn`
  (params (AxisValue :type "Float (single-precision)"))
  ;[1 1 1] Movement
  (`self.AddControllerYawInput` AxisValue))

(event `InputAction|Sprint`
  (params (Key :type "Key Structure"))
  ;[1 1 1] Sprint
  (:`Pressed`
    (`self.F_SprintSwitch` true))
  (:`Released`
    (`self.F_SprintSwitch` false)))

(event `InputAxis|LookUp`
  (params (AxisValue :type "Float (single-precision)"))
  ;[1 1 1] Movement
  (`self.AddControllerPitchInput` AxisValue))

(event `Server_ToggleSprint`
  (params (State :type Boolean))
  ;[1 1 1] Sprint
  (`self.F_SprintSwitch` State))

(event `InputAxis|MoveForward`
  (params (AxisValue :type "Float (single-precision)"))
  ;[1 1 1] Movement
  (`self.AddMovementInput` (`KismetMathLibrary.GetForwardVector` (`KismetMathLibrary.MakeRotator` 0.0 0.0 (.yaw (`self.GetControlRotation`)))) AxisValue))

(event `InputAxis|MoveRight`
  (params (AxisValue :type "Float (single-precision)"))
  ;[1 1 1] Movement
  (`self.AddMovementInput` (`KismetMathLibrary.GetRightVector` (`KismetMathLibrary.MakeRotator` 0.0 0.0 (.yaw (`self.GetControlRotation`)))) AxisValue))

(event `Multi_Rolling`
  (params (Mesh :type "SkeletalMeshComponent Object Reference") (Montage :type "AnimMontage Object Reference") (State :type Boolean))
  (bind _returnvalue (`SkeletalMeshComponent.GetAnimInstance` (`self.Mesh`)))
  ;[1 1 1] Rolling
  (if State
    (message `/Game/_Main/Interfaces/BPI_HeroAnimation.RollingState` _returnvalue true)
    (`|PlayMontage` Mesh Montage
      (:`OnCompleted`
        (`self.Server_Rolling` false)))
    (else
      (message `/Game/_Main/Interfaces/BPI_HeroAnimation.RollingState` _returnvalue false))))

(event `InputAction|Rolling`
  (params (Key :type "Key Structure"))
  ;[1 1 1] Rolling
  (:`Pressed`
    (if (and (not (`self.isRolling`)) (not (`self.isAttacking`)))
      (`self.Server_Rolling` true))))

(event `Server_Rolling`
  (params (isRolling :type Boolean))
  (bind _mesh (`self.Mesh`))
  ;[1 1 1] Rolling
  (if isRolling
    (set `self.isRolling` true)
    (`self.Multi_Rolling` _mesh "/Game/_Main/Player/GreystoneRoll_Montage.GreystoneRoll_Montage" true)
    (else
      (set `self.isRolling` false)
      (`self.Multi_Rolling` _mesh "/Game/_Main/Player/GreystoneRoll_Montage.GreystoneRoll_Montage"))))

(event `InputAction|Primary`
  (params (Key :type "Key Structure"))
  ;[1 1 1] Attacking
  (:`Pressed`
    (if (`.isWeaponEquiped_9_5D7CCDE8401D1A449ECAB9AAEDD6341F` (break `/Game/_Main/Player/S_EquipedItems` (`self.EquipedItems`)))
      (`self.Server_TryToActivateAbility` "NewEnumerator0"))))

(event `/Game/_Main/Interfaces/BPI_HeroCharacter.SetPickupInfo`
  (params (PickupObject :type "/Game/_Main/Items/BP_BasePickup Object Reference") (isOverlapped :type Boolean))
  (bind _returnvalue (`self.GetController`))
  ;[1 1 1] Set the pickup name to player's screen
  (if isOverlapped
    (bind _output_get (set `self.PickupItem` PickupObject))
    (bind _iteminfo_pickupname (break `/Game/_Main/Items/S_PickupInfo` (`/Game/_Main/Items/BP_BasePickup.ItemInfo` _output_get)))
    (message `/Game/_Main/Interfaces/BPI_PlayerControler.ShowPickupName` _returnvalue true _iteminfo_pickupname)
    (else
      (set `self.PickupItem` null)
      (message `/Game/_Main/Interfaces/BPI_PlayerControler.ShowPickupName` _returnvalue false ""))))

(event `InputAction|Secondary`
  (params (Key :type "Key Structure"))
  ;[1 1 1] Attacking
  (:`Pressed`
    (`self.Server_TryToActivateAbility` "NewEnumerator2")))

(event `Server_TryToActivateAbility`
  (params (Attacks :type "/Game/_Main/Player/E_PlayerAttacks Enum" :default "NewEnumerator0"))
  ;[1 1 1] Attacking
  (if (and (not (`self.isAttacking`)) (not (`self.isRolling`)))
    (switch `/Game/_Main/Player/E_PlayerAttacks` Attacks
      (:`NewEnumerator0`
        (set `self.isAttacking` true)
        (`self.Multi_PlayMontage` (`self.Mesh`) "/Game/_Main/Player/LightAttack_Montage.LightAttack_Montage")))))

(event `InputAction|Interact`
  (params (Key :type "Key Structure"))
  (:`Pressed`
    (`self.Server_InteractWithObject`)))

(event `Multi_PlayMontage`
  (params (InSkeletalMeshComponent :type "SkeletalMeshComponent Object Reference") (MontageToPlay :type "AnimMontage Object Reference") (StartingSection :type Name))
  ;[1 1 1] Attacking
  (`|PlayMontage` InSkeletalMeshComponent MontageToPlay 1.0 0.0 StartingSection
    (:`OnCompleted`
      (`self.Server_EndAttack`))))

(event `Server_InteractWithObject`
  (`self.PickupItem`
    (:`then`
      (`self.HandlePickup`))
    (:`else`)))

(event `Server_EndAttack`
  ;[1 1 1] Attacking
  (set `self.isAttacking` false))

(event `HandlePickup`
  (bind _pickupitem (`self.PickupItem`))
  (bind _picktype (message `/Game/_Main/Interfaces/BPI_Pickups.GetPickType` (`self.PickupItem`)))
  (switch `/Game/_Main/Items/E_PickupTypes` _picktype
    (:`NewEnumerator0`
      (`self.EquipedWeapon`
        (:`then`)
        (:`else`
          (`self.F_EquipWeapon` _pickupitem))))
    (:`NewEnumerator2`
      (`self.EquipedShield`
        (:`then`)
        (:`else`
          (`self.F_EquipShield` _pickupitem))))
    (:`NewEnumerator1`
      (`self.EquipedHelmet`
        (:`then`)
        (:`else`
          (`self.F_EquipHelmet` _pickupitem))))))

(fn `F_EquipHelmet`
  (params (EquipedHelmet :type "Actor Object Reference"))
  (if (not (`.isHelmetEquiped_7_CC25A5204D2133C2AA2A0BA963BDCE39` (break `/Game/_Main/Player/S_EquipedItems` (`self.EquipedItems`))))
    (set `self.EquipedHelmet` EquipedHelmet)
    (setmembers `/Game/_Main/Player/S_EquipedItems` :`StructRef` (`self.EquipedItems`) :`isHelmetEquiped` true)))

(fn `F_EquipShield`
  (params (EquipedShield :type "Actor Object Reference"))
  (if (not (`.isShieldEquiped_10_20DA4A714939602FCC83E9A5DB5CF8E6` (break `/Game/_Main/Player/S_EquipedItems` (`self.EquipedItems`))))
    (set `self.EquipedShield` EquipedShield)
    (setmembers `/Game/_Main/Player/S_EquipedItems` :`StructRef` (`self.EquipedItems`) :`isShieldEquiped` true)))

(fn `F_EquipWeapon`
  (params (WeaponToEquip :type "Actor Object Reference"))
  (if (not (`.isWeaponEquiped_9_5D7CCDE8401D1A449ECAB9AAEDD6341F` (break `/Game/_Main/Player/S_EquipedItems` (`self.EquipedItems`))))
    (set `self.EquipedWeapon` WeaponToEquip)
    (setmembers `/Game/_Main/Player/S_EquipedItems` :`StructRef` (`self.EquipedItems`) :`isWeaponEquiped` true)))

(fn `F_SprintSwitch`
  (params (SprintState :type Boolean))
  (locals (LocalSprint :type Boolean))
  (bind _charactermovement (`self.CharacterMovement`))
  (bind _charactermovement_2 (`self.CharacterMovement`))
  (bind _output_get (set `local.LocalSprint` SprintState))
  (`/Engine/EditorBlueprintResources/ActorMacros.Switch Has Authority`
    (:`Authority`
      (if (`local.LocalSprint`)
        (set `CharacterMovementComponent.MaxWalkSpeed` (`self.SprintSpeed`) _charactermovement)
        (set `self.isSprinting` true)
        (else
          (set `CharacterMovementComponent.MaxWalkSpeed` (`self.JogSpeed`) _charactermovement)
          (set `self.isSprinting` false)))
      (return))
    (:`Remote`
      (`self.Server_ToggleSprint` _output_get)
      (if (`local.LocalSprint`)
        (set `CharacterMovementComponent.MaxWalkSpeed` (`self.SprintSpeed`) _charactermovement_2)
        (else
          (set `CharacterMovementComponent.MaxWalkSpeed` (`self.JogSpeed`) _charactermovement_2)))
      (return))))

(fn `OnRep_EquipedHelmet`
  (bind _equipedhelmet (`self.EquipedHelmet`))
  (`self.K2_AttachToComponent` _equipedhelmet (`self.Mesh`) "Helmet" "SnapToTarget" "SnapToTarget" "KeepRelative" true)
  (message `/Game/_Main/Interfaces/BPI_Pickups.DisablePhysics` _equipedhelmet))

(fn `OnRep_EquipedShield`
  (bind _equipedshield (`self.EquipedShield`))
  (`self.K2_AttachToComponent` _equipedshield (`self.Mesh`) "shield" "SnapToTarget" "SnapToTarget" "KeepRelative" true)
  (message `/Game/_Main/Interfaces/BPI_Pickups.DisablePhysics` _equipedshield))

(fn `OnRep_EquipedWeapon`
  (bind _equipedweapon (`self.EquipedWeapon`))
  (`self.K2_AttachToComponent` _equipedweapon (`self.Mesh`) "Weapon_R" "SnapToTarget" "SnapToTarget" "KeepRelative" true)
  (message `/Game/_Main/Interfaces/BPI_Pickups.DisablePhysics` _equipedweapon))

(fn `OnRep_isSprinting`
  (bind _returnvalue (`SkeletalMeshComponent.GetAnimInstance` (`self.Mesh`)))
  (if (`self.isSprinting`)
    (message `/Game/_Main/Interfaces/BPI_HeroAnimation.SprintState` _returnvalue true)
    (else
      (message `/Game/_Main/Interfaces/BPI_HeroAnimation.SprintState` _returnvalue false))))

(fn `UserConstructionScript`
  (`parent.UserConstructionScript`))