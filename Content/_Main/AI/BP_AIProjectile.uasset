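; BP_AIProjectile is an AI projectile that damages actors tagged Player on contact.
; On the server, a sphere overlap sets a hit flag, applies damage with the projectile's owner as causer, then destroys the projectile.
; The Destroyed event checks that flag and calls Multi_SpawnFX to spawn the hit emitter at the projectile's location, so only player hits produce the effect.
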(event `self.Sphere.OnComponentBeginOverlap`
  (params (OverlappedComponent :type "PrimitiveComponent Object Reference") (OtherActor :type "Actor Object Reference") (OtherComp :type "PrimitiveComponent Object Reference") (OtherBodyIndex :type Integer) (bFromSweep :type Boolean) (SweepResult :type "HitResult Structure (by ref)"))
  (`/Engine/EditorBlueprintResources/ActorMacros.Switch Has Authority`
    (:`Authority`
      (if (`self.ActorHasTag` OtherActor "Player")
        (set `self.isHit` true)
        (`GameplayStatics.ApplyDamage` OtherActor (`self.Damage`) null (`self.GetOwner`) "/Script/Engine.DamageType")
        (`self.K2_DestroyActor`)))))

(event `self.ReceiveDestroyed`
  (if (`self.isHit`)
    (`self.Multi_SpawnFX` (`self.HitEmmiter`) (`self.K2_GetActorLocation`))))

(event `Multi_SpawnFX`
  (params (EmitterTemplate :type "ParticleSystem Object Reference") (Location :type "Vector Structure"))
  (`GameplayStatics.SpawnEmitterAttached` EmitterTemplate null "None" Location))

(fn `UserConstructionScript`)